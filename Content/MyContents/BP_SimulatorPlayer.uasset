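; BP_SimulatorPlayer is the first-person player vehicle of a driving simulator, driven entirely by values read each Tick from BP_SimulatorGameModeBase.
; Hand coordinates and WheelAngle pose both hands and the steering wheel, while IsHandle toggles the hands' black unlit material.
; A non-zero Control moves the actor along its heading at Speed, steering by WheelAngle only while moving.
; ClipedXdiff offsets the camera's yaw from the actor's, even when stationary.
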(event EventBeginPlay
  (bind _asbp_simulator_game_mode_base (Utilities|Casting|CastToBP_SimulatorGameModeBase (Game|GetGameMode))))

(event Collision|EventActorBeginOverlap
  (params (OtherActor :type Actor%20Object%20Reference)))

(event EventTick
  (params (DeltaSeconds :type Float%20%28single-precision%29))
  (bind _handright (Variables|Default|GetHandRight))
  (bind _handleft (Variables|Default|GetHandLeft))
  ;[1 1 1] 손이동처리
  (Utilities|FlowControl|Sequence
    (:then_0
      (if (Variables|/Script/CarSimulator.SimulatorGameModeBase|Getis_handle (stale EventBeginPlay _asbp_simulator_game_mode_base))
        (Rendering|Material|SetMaterial _handleft 0 "/Engine/EngineDebugMaterials/BlackUnlitMaterial.BlackUnlitMaterial")
        (Rendering|Material|SetMaterial _handright 0 "/Engine/EngineDebugMaterials/BlackUnlitMaterial.BlackUnlitMaterial")
        (else
          (Rendering|Material|SetMaterial _handleft 0 0)
          (Rendering|Material|SetMaterial _handright 0 0))))
    (:then_1
      (Transformation|SetRelativeLocationAndRotation _handleft (Math|Vector|MakeVector 37.0 (- (/ (Variables|/Script/CarSimulator.SimulatorGameModeBase|Gethand_left_x (stale EventBeginPlay _asbp_simulator_game_mode_base)) 6.0) 93.0) (- 8e+01 (/ (Variables|/Script/CarSimulator.SimulatorGameModeBase|Gethand_left_y (stale EventBeginPlay _asbp_simulator_game_mode_base)) 6.0))) (Math|Rotator|MakeRotator 0.0 (Variables|/Script/CarSimulator.SimulatorGameModeBase|GetwheelAngle (stale EventBeginPlay _asbp_simulator_game_mode_base)) 9e+01) false false)
      (Transformation|SetRelativeLocationAndRotation _handright (Math|Vector|MakeVector 37.0 (- (/ (Variables|/Script/CarSimulator.SimulatorGameModeBase|Gethand_right_x (stale EventBeginPlay _asbp_simulator_game_mode_base)) 6.0) 93.0) (- 8e+01 (/ (Variables|/Script/CarSimulator.SimulatorGameModeBase|Gethand_right_y (stale EventBeginPlay _asbp_simulator_game_mode_base)) 6.0))) (Math|Rotator|MakeRotator 0.0 (Variables|/Script/CarSimulator.SimulatorGameModeBase|GetwheelAngle (stale EventBeginPlay _asbp_simulator_game_mode_base)) 9e+01) false false)
      ;[1 1 1] 카메라 회전로직
      (Transformation|SetRelativeRotation (Variables|Default|GetSteeringWheel) (Math|Rotator|MakeRotator 0.0 (Variables|/Script/CarSimulator.SimulatorGameModeBase|GetwheelAngle (stale EventBeginPlay _asbp_simulator_game_mode_base)) 9e+01) false false)
      ;[1 1 1] 차량 이동 로직
      (if (== (Variables|/Script/CarSimulator.SimulatorGameModeBase|Getcontrol (stale EventBeginPlay _asbp_simulator_game_mode_base)) 0)
        (Transformation|SetWorldRotation (Variables|Default|GetfpCamComp) (Math|Rotator|MakeRotator 0.0 0.0 (+ (* (Variables|/Script/CarSimulator.SimulatorGameModeBase|Getcliped_xdiff (stale EventBeginPlay _asbp_simulator_game_mode_base)) -1.0) (.yaw (Transformation|GetActorRotation)))) false false)
        (else
          (Transformation|SetActorLocationAndRotation (+ (Transformation|GetActorLocation) (* (Math|Vector|Normalize (Math|Vector|GetForwardVector (Math|Rotator|MakeRotator 0.0 0.0 (+ (* (Variables|/Script/CarSimulator.SimulatorGameModeBase|GetwheelAngle (stale EventBeginPlay _asbp_simulator_game_mode_base)) -0.02) (.yaw (Transformation|GetActorRotation)))))) (Variables|Default|GetSpeed) (Variables|/Script/CarSimulator.SimulatorGameModeBase|Getcontrol (stale EventBeginPlay _asbp_simulator_game_mode_base)))) (Math|Rotator|MakeRotator 0.0 0.0 (+ (* (Variables|/Script/CarSimulator.SimulatorGameModeBase|GetwheelAngle (stale EventBeginPlay _asbp_simulator_game_mode_base)) -0.02) (.yaw (Transformation|GetActorRotation)))))
          (Transformation|SetWorldRotation (Variables|Default|GetfpCamComp) (Math|Rotator|MakeRotator 0.0 0.0 (+ (* (Variables|/Script/CarSimulator.SimulatorGameModeBase|Getcliped_xdiff (stale EventBeginPlay _asbp_simulator_game_mode_base)) -1.0) (.yaw (Transformation|GetActorRotation)))) false false))))))

(fn ConstructionScript)