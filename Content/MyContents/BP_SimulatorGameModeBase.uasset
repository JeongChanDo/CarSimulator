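; BP_SimulatorGameModeBase is the simulator's game mode, showing a periodically refreshed image feed on screen.
; On BeginPlay it creates BP_MainWidget and adds it to the viewport.
; Tick accumulates time, and once it exceeds SpendTime it calls ReadFrame, resets the timer and pushes ImageTexture into the widget's image.
; A debug print of Control and WheelAngle is left unconnected.
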(event EventBeginPlay
  (bind _returnvalue (UserInterface|CreateWidget "/Game/MyContents/BP_MainWidget.BP_MainWidget_C"))
  (UserInterface|Viewport|AddtoViewport _returnvalue 0)
  (Variables|Default|SetMainUI _returnvalue))

(event EventTick
  (params (DeltaSeconds :type Float%20%28single-precision%29))
  (if (> (Variables|Default|GetCurrentTime) (Variables|Default|GetSpendTime))
    (Class|SimulatorGameModeBase|ReadFrame)
    (Variables|Default|SetCurrentTime 0.0)
    (Appearance|SetBrushfromTexture (Variables|/Game/MyContents/BP_MainWidget.BP_MainWidget_C|GetimageWidget (Variables|Default|GetMainUI)) (Variables|Default|GetimageTexture) false)
    (else
      (Variables|Default|SetCurrentTime (+ DeltaSeconds (Variables|Default|GetCurrentTime))))))

(fn ConstructionScript)